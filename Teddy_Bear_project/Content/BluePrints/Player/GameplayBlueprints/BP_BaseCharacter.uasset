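; BP_BaseCharacter is the player character Blueprint, handling look, movement, sprint, crouch, jumping with double-jump tracking, and air dash through input actions.
; Interact sphere-traces around the character and sends InteractMessage to hit actors implementing BPI_Interaction.
; Air dash zeroes gravity, launches along movement input or flattened camera forward, and sets a timer.
; Landing re-arms the dash and resets jump state, with 2D sounds accompanying actions.
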(event Input|EnhancedActionEvents|EnhancedInputActionIA_Interact
  (params (ActionValue :type Boolean) (ElapsedSeconds :type Float%20%28double-precision%29) (TriggeredSeconds :type Float%20%28double-precision%29) (InputAction :type Input%20Action%20Object%20Reference :default "/Game/Inputs/InputsActions/IA_Interact.IA_Interact"))
  (Audio|PlaySound2D "/Game/Sounds/Interact.Interact" 1.0 1.0 0.0 0 0))

(event Input|EnhancedActionEvents|EnhancedInputActionIA_AirDash
  (params (ActionValue :type Boolean) (ElapsedSeconds :type Float%20%28double-precision%29) (TriggeredSeconds :type Float%20%28double-precision%29) (InputAction :type Input%20Action%20Object%20Reference :default "/Game/Inputs/InputsActions/IA_AirDash.IA_AirDash"))
  (:Started
    (Audio|PlaySound2D "/Game/Sounds/Dash.Dash" 1.0 1.0 0.0 0 0)))

(event Input|EnhancedActionEvents|EnhancedInputActionIA_AirDash
  (params (ActionValue :type Boolean) (ElapsedSeconds :type Float%20%28double-precision%29) (TriggeredSeconds :type Float%20%28double-precision%29) (InputAction :type Input%20Action%20Object%20Reference :default "/Game/Inputs/InputsActions/IA_AirDash.IA_AirDash"))
  (:Started
    (if (Variables|Default|GetCanAirDash)
      (CallFunction|AirDash)
      (Variables|Default|SetCanAirDash false)
      (Variables|Default|SetisAirDashing true))))

(event Input|EnhancedActionEvents|EnhancedInputActionIA_MoveForward
  (params (ActionValue :type Float%20%28double-precision%29) (ElapsedSeconds :type Float%20%28double-precision%29) (TriggeredSeconds :type Float%20%28double-precision%29) (InputAction :type Input%20Action%20Object%20Reference :default "/Game/Inputs/InputsActions/IA_MoveForward.IA_MoveForward"))
  (:Triggered
    (Pawn|Input|AddMovementInput (Math|Vector|GetForwardVector (Math|Rotator|MakeRotator 0.0 0.0 (.yaw (Pawn|GetControlRotation :!class /Script/Engine.Pawn)))) ActionValue false)))

(event Input|EnhancedActionEvents|EnhancedInputActionIA_Look
  (params (ActionValue :type Vector%202D%20Structure) (ElapsedSeconds :type Float%20%28double-precision%29) (TriggeredSeconds :type Float%20%28double-precision%29) (InputAction :type Input%20Action%20Object%20Reference :default "/Game/Inputs/InputsActions/IA_Look.IA_Look"))
  (Pawn|Input|AddControllerYawInput (.x ActionValue))
  (Pawn|Input|AddControllerPitchInput (.y ActionValue)))

(event Input|EnhancedActionEvents|EnhancedInputActionIA_MoveRight
  (params (ActionValue :type Float%20%28double-precision%29) (ElapsedSeconds :type Float%20%28double-precision%29) (TriggeredSeconds :type Float%20%28double-precision%29) (InputAction :type Input%20Action%20Object%20Reference :default "/Game/Inputs/InputsActions/IA_MoveRight.IA_MoveRight"))
  (Pawn|Input|AddMovementInput (Math|Vector|GetRightVector (Math|Rotator|MakeRotator 0.0 0.0 (.yaw (Pawn|GetControlRotation :!class /Script/Engine.Pawn)))) ActionValue false))

(event Input|EnhancedActionEvents|EnhancedInputActionIA_Sprint
  (params (ActionValue :type Boolean) (ElapsedSeconds :type Float%20%28double-precision%29) (TriggeredSeconds :type Float%20%28double-precision%29) (InputAction :type Input%20Action%20Object%20Reference :default "/Game/Inputs/InputsActions/IA_Sprint.IA_Sprint"))
  (bind _charactermovement (Variables|Character|GetCharacterMovement))
  (:Triggered
    (Variables|/Script/Engine.CharacterMovementComponent|SetMaxWalkSpeed _charactermovement 1e+03))
  (:Canceled
    (Variables|/Script/Engine.CharacterMovementComponent|SetMaxWalkSpeed _charactermovement 5e+02 :!label _label))
  (:Completed
    (goto _label)))

(event Input|EnhancedActionEvents|EnhancedInputActionIA_Crouch
  (params (ActionValue :type Boolean) (ElapsedSeconds :type Float%20%28double-precision%29) (TriggeredSeconds :type Float%20%28double-precision%29) (InputAction :type Input%20Action%20Object%20Reference :default "/Game/Inputs/InputsActions/IA_Crouch.IA_Crouch"))
  (:Started
    (Character|Crouch)
    (Variables|Default|SetisCrouching true))
  (:Completed
    (Character|UnCrouch)
    (Variables|Default|SetisCrouching false)))

(event Input|EnhancedActionEvents|EnhancedInputActionIA_Jump
  (params (ActionValue :type Boolean) (ElapsedSeconds :type Float%20%28double-precision%29) (TriggeredSeconds :type Float%20%28double-precision%29) (InputAction :type Input%20Action%20Object%20Reference :default "/Game/Inputs/InputsActions/IA_Jump.IA_Jump"))
  (:Triggered
    (Character|Jump))
  (:Started
    (Math|Integer|IncrementInt (Variables|Default|GetjumpCount)
      (:%20%20
        (if (== (Variables|Default|GetjumpCount) 2)
          (Variables|Default|SetcanDoubleJump true)
          (Audio|PlaySound2D "/Game/Sounds/DoubleJump.DoubleJump" 1.0 1.0 0.0 0 0)
          (else
            (Variables|Default|SetcanDoubleJump false)
            (Audio|PlaySound2D "/Game/Sounds/Jump.Jump" 1.0 1.0 0.0 0 0))))))
  (:Canceled
    (Character|StopJumping :!label _label))
  (:Completed
    (goto _label)))

(event Input|EnhancedActionEvents|EnhancedInputActionIA_Interact
  (params (ActionValue :type Boolean) (ElapsedSeconds :type Float%20%28double-precision%29) (TriggeredSeconds :type Float%20%28double-precision%29) (InputAction :type Input%20Action%20Object%20Reference :default "/Game/Inputs/InputsActions/IA_Interact.IA_Interact"))
  (bind _returnvalue (Transformation|GetActorLocation))
  (bind (_outhits _returnvalue_2) (Collision|MultiSphereTraceForObjects _returnvalue _returnvalue 1e+02 (Utilities|Array|MakeArray "ObjectTypeQuery1" "ObjectTypeQuery2") false 0 "None"))
  (if _returnvalue_2
    (for _array_element _outhits
      (if (Utilities|DoesObjectImplementInterface (.HitActor (Collision|BreakHitResult _array_element)) "/Game/LevelConstructionElements/BPI_Interaction.BPI_Interaction_C")
        (Class|BPIInteraction|Interact(Message) (.HitActor (Collision|BreakHitResult _array_element)))))))

(event EventOnLanded
  (params (Hit :type Hit%20Result%20Structure%20%28by%20ref%29))
  (Variables|Default|SetCanAirDash true)
  (Variables|Default|SetjumpCount 0)
  (Variables|Default|SetcanDoubleJump false)
  (Audio|PlaySound2D "/Game/Sounds/Land.Land" 1.0 1.0 0.0 0 0))

(fn ConstructionScript)

(fn AirDash
  (Variables|/Script/Engine.CharacterMovementComponent|SetGravityScale (Variables|Character|GetCharacterMovement) 0.0)
  (Character|LaunchCharacter (* (CallFunction|GetAirDashVector) (Variables|Default|GetAirDashSpeed)) true true)
  (Utilities|Time|SetTimerbyEvent (EventDispatchers|CreateEvent :!event EndAirDash) (Variables|Default|GetTime)))

(fn EndAirDash
  (Variables|/Script/Engine.CharacterMovementComponent|SetGravityScale (Variables|Character|GetCharacterMovement) 1.0)
  (Variables|Default|SetisAirDashing false))

(fn GetAirDashVector
  (bind _returnvalue (Class|Pawn|GetLastMovementInputVector))
  (return (Math|Vector|SelectVector _returnvalue (* (Transformation|GetActorForwardVector (Game|GetPlayerCameraManager 0)) "1.000000,1.000000,0.000000") (> (Math|Vector|VectorLength _returnvalue) 0.5))))