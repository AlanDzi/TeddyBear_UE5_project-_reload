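; BP_BaseMode is a base mode Blueprint, apparently the game mode, that handles player respawning through its RespawnPlayer event.
; The event destroys the current player character, then spawns a BP_BaseCharacter at LastCheckPoint's POS location and rotation and has player controller 0 possess it.
; Without a valid checkpoint, it spawns at the default transform and calls Possess with no pawn connected.
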(event Custom|RespawnPlayer
  (Actor|DestroyActor (Game|GetPlayerCharacter 0))
  (bind _lastcheckpoint (Variables|Default|GetLastCheckPoint)
    (:then
      (bind _returnvalue (Game|SpawnActorfromClass "/Game/BluePrints/Player/GameplayBlueprints/BP_BaseCharacter.BP_BaseCharacter_C" (Math|Transform|MakeTransform (.location (Transformation|GetWorldTransform (Variables|/Game/BluePrints/BP_CheckPoint.BP_CheckPoint_C|GetPOS _lastcheckpoint))) (.rotation (Transformation|GetWorldTransform (Variables|/Game/BluePrints/BP_CheckPoint.BP_CheckPoint_C|GetPOS _lastcheckpoint))) "1.000000,1.000000,1.000000") "AlwaysSpawn" "MultiplyWithRoot" 0 0))
      (Pawn|Possess (Game|GetPlayerController 0) _returnvalue))
    (:else
      (Game|SpawnActorfromClass "/Game/BluePrints/Player/GameplayBlueprints/BP_BaseCharacter.BP_BaseCharacter_C" (Math|Transform|MakeTransform "0, 0, 0" "0, 0, 0" "1.000000,1.000000,1.000000") "AlwaysSpawn" "MultiplyWithRoot" 0 0)
      (Pawn|Possess (Game|GetPlayerController 0)))))

(fn ConstructionScript)